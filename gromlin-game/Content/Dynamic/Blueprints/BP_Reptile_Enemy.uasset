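; BP_Reptile_Enemy is a patrolling flipbook enemy that can be stomped by the player.
; WallDetector and LedgeDetector overlaps flip it around, while MoveForward drives it along its facing direction.
; Hitbox contact bounces the player upward and sets a timed Hit state that halts MoveForward and swaps in the stomp flipbook on Tick.
; Hurtbox contact calls BeenHurt on the player.
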(event OnComponentBeginOverlap(WallDetector)
  (params (OverlappedComponent :type Primitive%20Component%20Object%20Reference) (OtherActor :type Actor%20Object%20Reference) (OtherComp :type Primitive%20Component%20Object%20Reference) (OtherBodyIndex :type Integer) (bFromSweep :type Boolean) (SweepResult :type Hit%20Result%20Structure%20%28by%20ref%29))
  (CallFunction|TurnChar))

(event OnComponentEndOverlap(LedgeDetector)
  (params (OverlappedComponent :type Primitive%20Component%20Object%20Reference) (OtherActor :type Actor%20Object%20Reference) (OtherComp :type Primitive%20Component%20Object%20Reference) (OtherBodyIndex :type Integer))
  (CallFunction|TurnChar))

(event OnComponentBeginOverlap(Hitbox)
  (params (OverlappedComponent :type Primitive%20Component%20Object%20Reference) (OtherActor :type Actor%20Object%20Reference) (OtherComp :type Primitive%20Component%20Object%20Reference) (OtherBodyIndex :type Integer) (bFromSweep :type Boolean) (SweepResult :type Hit%20Result%20Structure%20%28by%20ref%29))
  (bind _asbp_player (Utilities|Casting|CastToBP_Player OtherActor))
  (Character|LaunchCharacter _asbp_player "0.000000,0.000000,1300.000000" false true)
  (Variables|Default|SetHit? true)
  (Utilities|FlowControl|Delay 4.116667)
  (Variables|Default|SetHit? false))

(event OnComponentBeginOverlap(Hurtbox)
  (params (OverlappedComponent :type Primitive%20Component%20Object%20Reference) (OtherActor :type Actor%20Object%20Reference) (OtherComp :type Primitive%20Component%20Object%20Reference) (OtherBodyIndex :type Integer) (bFromSweep :type Boolean) (SweepResult :type Hit%20Result%20Structure%20%28by%20ref%29))
  (bind _asbp_player (Utilities|Casting|CastToBP_Player OtherActor))
  (Default|BeenHurt _asbp_player))

(event Custom|Move%20Forward
  (if (Variables|Default|GetHit?)
    (Variables|/Script/Engine.MovementComponent|SetVelocity (Variables|Character|GetCharacterMovement) "0, 0, 0")
    (else
      (Pawn|Input|AddMovementInput (Transformation|GetActorForwardVector) 1.0 false))))

(event Custom|Update%20Animation
  (Sprite|SetFlipbook (Variables|Default|GetSprite) (select (Variables|Default|GetHit?) "/Game/Static/Sprites/Enemies/Sewers/FB_Reptile_Walk_Stomop.FB_Reptile_Walk_Stomop" "/Game/Static/Sprites/Enemies/Sewers/FB_Reptile_Walk.FB_Reptile_Walk")))

(event EventTick
  (params (DeltaSeconds :type Float%20%28single-precision%29))
  (CallFunction|UpdateAnimation))

(fn ConstructionScript)

(fn TurnChar
  (Transformation|SetActorRotation (Math|Rotator|CombineRotators (Transformation|GetActorRotation) "0.000000,180.000000,0.000000")))