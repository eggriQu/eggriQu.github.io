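; BP_Level is a level actor that sets the environment tile map and handles the transition on level completion.
; On BeginPlay, SetLevel uses the Level variable to put either the sewers or housing estate map on the TMSewers component.
; LevelComplete destroys the children of LevelObjects, repeating until none remain, then opens the fixed LEVEL2 map after a short delay.
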(event Custom|Level%20Complete
  (bind _level_objects (Variables|Default|GetLevel%20Objects))
  (bind _children (Components|GetChildrenComponents _level_objects false))
  (for _array_element _children :!label _label
    (Components|DestroyComponent _array_element))
  (if (Utilities|Array|IsEmpty _children)
    (Utilities|FlowControl|Delay 2.0)
    (Game|OpenLevel(byObjectReference) "/Game/Dynamic/Maps/LEVEL2.LEVEL2")
    (else
      (goto _label))))

(event Custom|Set%20Level
  (Class|PaperTileMapComponent|SetTileMap (Variables|Default|GetTM_Sewers) (Utilities|Select :Index (Variables|Default|GetLevel) :Option%200 "/Game/Dynamic/Tilemaps/TM_Sewers.TM_Sewers" :Option%201 "/Game/Dynamic/Tilemaps/TM_Housing_Estate.TM_Housing_Estate")))

(event EventBeginPlay
  (CallFunction|SetLevel))

(event Collision|EventActorBeginOverlap
  (params (OtherActor :type Actor%20Object%20Reference)))

(event EventTick
  (params (DeltaSeconds :type Float%20%28single-precision%29)))

(fn ConstructionScript)