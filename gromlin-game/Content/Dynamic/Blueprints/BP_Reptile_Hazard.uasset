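; Stationary 2D reptile hazard that rises when BP_Player enters its detection range and spits projectiles at them, then sinks when they leave.
; A delay loop repeats the attack, spawning BP_Reptile_Spit with an impulse aimed at the player.
; Touching its hitbox launches the player upward and temporarily stuns the reptile, lowering its sprite.
; Tick selects flipbooks from the attack and hit flags and turns the actor by the player's X position.
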(event OnComponentBeginOverlap(DetectionRange)
  (params (OverlappedComponent :type Primitive%20Component%20Object%20Reference) (OtherActor :type Actor%20Object%20Reference) (OtherComp :type Primitive%20Component%20Object%20Reference) (OtherBodyIndex :type Integer) (bFromSweep :type Boolean) (SweepResult :type Hit%20Result%20Structure%20%28by%20ref%29))
  (Utilities|Casting|CastToBP_Player OtherActor)
  (if (not (Variables|Default|GetHit?))
    (Variables|Default|SetDetected%20Player? true)
    (Components|MoveComponentTo (Variables|Default|GetSprite) "0.000000,0.000000,50.000000" "0, 0, 0" false false 0.2 false)
    (Utilities|FlowControl|Delay 0.783333)
    (CallFunction|Attack :!label _label)
    (Utilities|FlowControl|Delay 1.5)
    (if (Variables|Default|GetDetected%20Player?)
      (goto _label))))

(event OnComponentEndOverlap(DetectionRange)
  (params (OverlappedComponent :type Primitive%20Component%20Object%20Reference) (OtherActor :type Actor%20Object%20Reference) (OtherComp :type Primitive%20Component%20Object%20Reference) (OtherBodyIndex :type Integer))
  (Utilities|Casting|CastToBP_Player OtherActor)
  (if (not (Variables|Default|GetHit?))
    (Variables|Default|SetDetected%20Player? false)
    (Components|MoveComponentTo (Variables|Default|GetSprite) "0.000000,0.000000,-50.000000" "0, 0, 0" false false 0.2 false)))

(event OnComponentBeginOverlap(Hitbox)
  (params (OverlappedComponent :type Primitive%20Component%20Object%20Reference) (OtherActor :type Actor%20Object%20Reference) (OtherComp :type Primitive%20Component%20Object%20Reference) (OtherBodyIndex :type Integer) (bFromSweep :type Boolean) (SweepResult :type Hit%20Result%20Structure%20%28by%20ref%29))
  (bind _asbp_player (Utilities|Casting|CastToBP_Player OtherActor))
  (Character|LaunchCharacter _asbp_player "0.000000,0.000000,1400.000000" false true)
  (Variables|Default|SetHit? true)
  (Variables|Default|SetDetected%20Player? false)
  (Sprite|SetFlipbook (Variables|Default|GetSprite) "/Game/Static/Sprites/Enemies/Sewers/FB_Reptile_Stomp.FB_Reptile_Stomp")
  (Components|MoveComponentTo (Variables|Default|GetSprite) "0.000000,0.000000,-50.000000" "0, 0, 0" false false 1.433333 false)
  (Sprite|SetFlipbook (Variables|Default|GetSprite) "/Game/Static/Sprites/Enemies/Sewers/FB_Reptile_Hazard.FB_Reptile_Hazard")
  (Utilities|FlowControl|Delay 2.0)
  (Variables|Default|SetHit? false)
  (if (Variables|Default|GetDetected%20Player?)
    (Components|MoveComponentTo (Variables|Default|GetSprite) "0.000000,0.000000,10.000000" "0, 0, 0" false false 0.683333 false)))

(event Custom|Attack
  (bind _returnvalue (Game|Player|GetPlayerPawn 0))
  (bind _projectile_source (Variables|Default|GetProjectile%20Source))
  (bind _returnvalue_2 (Transformation|GetWorldLocation _projectile_source))
  (bind _returnvalue_3 (Transformation|GetActorLocation _returnvalue))
  (bind _returnvalue_4 (Math|Rotator|FindLookatRotation _returnvalue_2 _returnvalue_3))
  (if (Math|Boolean|ANDBoolean (Variables|Default|GetDetected%20Player?) (not (Variables|Default|GetHit?)) (not (Variables|Default|GetAttacking?)))
    (bind _returnvalue_5 (Game|SpawnActorfromClass "/Game/Dynamic/Blueprints/BP_Reptile_Spit.BP_Reptile_Spit_C" (Math|Transform|MakeTransform (.location (Math|Transform|MakeTransform _returnvalue_2)) _returnvalue_4 "1.000000,1.000000,1.000000") "Undefined" "MultiplyWithRoot" 0 0))
    (Physics|AddImpulse (Variables|/Game/Dynamic/Blueprints/BP_Reptile_Spit.BP_Reptile_Spit_C|GetBox _returnvalue_5) (* (Math|Vector|Normalize (Math|Vector|GetForwardVector _returnvalue_4)) 3.5e+04) "None" false)
    (Variables|Default|SetAttacking? true)
    (Utilities|FlowControl|Delay 0.783333)
    (Variables|Default|SetAttacking? false)))

(event Custom|Update%20Animation
  (bind _hit_ (Variables|Default|GetHit?))
  (if (and (Variables|Default|GetAttacking?) (not _hit_))
    (Sprite|SetFlipbook (Variables|Default|GetSprite) "/Game/Static/Sprites/Enemies/Sewers/FB_Reptile_Attack.FB_Reptile_Attack")
    (elif (not _hit_)
      (Sprite|SetFlipbook (Variables|Default|GetSprite) "/Game/Static/Sprites/Enemies/Sewers/FB_Reptile_Hazard.FB_Reptile_Hazard"))))

(event Custom|Update%20Rotation
  (if (< (.x (Transformation|GetActorLocation (Game|Player|GetPlayerPawn 0))) (.x (Transformation|GetWorldLocation (Variables|Collision|GetCapsuleComponent))))
    (Transformation|SetActorRotation "0.000000,0.000000,0.000000")
    (else
      (Transformation|SetActorRotation "0.000000,180.000000,0.000000"))))

(event EventBeginPlay)

(event Collision|EventActorBeginOverlap
  (params (OtherActor :type Actor%20Object%20Reference)))

(event EventTick
  (params (DeltaSeconds :type Float%20%28single-precision%29))
  (CallFunction|UpdateAnimation)
  (CallFunction|UpdateRotation))

(fn ConstructionScript)

(fn TurnChar
  (Transformation|SetActorRotation (Math|Rotator|CombineRotators (Transformation|GetActorRotation) "0.000000,180.000000,0.000000")))