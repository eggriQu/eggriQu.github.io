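; BP_Pipe_Hazard is a 2D pipe hazard that repeatedly drips a projectile straight down.
; An endless delay loop started on BeginPlay switches the sprite from still to dripping flipbook, then spawns a projectile at the sprite's X and Z position as the drip ends.
; It reuses BP_Reptile_Spit as the drop, rotated and scaled, and launches it with a downward velocity-change impulse on its box.
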(event EventBeginPlay
  (bind _sprite (Variables|Default|GetSprite))
  (bind _returnvalue (Transformation|GetWorldLocation _sprite))
  (Utilities|FlowControl|Delay 1.5 :!label _label)
  (Sprite|SetFlipbook (Variables|Default|GetSprite) "/Game/Static/Placeholder_Sprites/Enemies/FB_Pipe_Dripping.FB_Pipe_Dripping")
  (Utilities|FlowControl|Delay 0.383333)
  (bind _returnvalue_2 (Game|SpawnActorfromClass "/Game/Dynamic/Blueprints/BP_Reptile_Spit.BP_Reptile_Spit_C" (Math|Transform|MakeTransform (Math|Vector|MakeVector (.x _returnvalue) 0.0 (.z _returnvalue)) "-90.000000,0.000000,0.000000" "1.500000,1.000000,1.500000") "Undefined" "MultiplyWithRoot" 0 0))
  (Sprite|SetFlipbook (Variables|Default|GetSprite) "/Game/Static/Placeholder_Sprites/Enemies/FB_Pipe_Still.FB_Pipe_Still")
  (Physics|AddImpulse (Variables|/Game/Dynamic/Blueprints/BP_Reptile_Spit.BP_Reptile_Spit_C|GetBox _returnvalue_2) "0.000000,0.000000,-900.000000" "None" true)
  (goto _label))

(fn ConstructionScript)